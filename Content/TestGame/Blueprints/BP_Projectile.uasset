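; BP_Projectile is a projectile actor that reports what it hits and then destroys itself.
; Its Sphere1 component ignores the owner while moving and on hit events.
; A hit on any other actor fires the OnProjectileHit dispatcher with that actor and the hit result, leaving the response to listeners.
; Its health, heal and damage functions are stubs returning zero or false.
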(event OnComponentHit(Sphere1)
  (params (HitComponent :type Primitive%20Component%20Object%20Reference) (OtherActor :type Actor%20Object%20Reference) (OtherComp :type Primitive%20Component%20Object%20Reference) (NormalImpulse :type Vector :default "0, 0, 0") (Hit :type Hit%20Result%20Structure%20%28by%20ref%29))
  (if (not (== OtherActor (Components|GetOwner)))
    (Default|CallOnProjectileHit OtherActor Hit)
    (Actor|DestroyActor)))

(event EventBeginPlay
  (Collision|IgnoreActorwhenMoving (Variables|Components|GetSphere1) (Components|GetOwner) true))

(fn ConstructionScript)

(fn GetCurrentHealth
  (return 0.0))

(fn GetMaxHealth
  (return 0.0))

(fn Heal
  (params (Amount :type Float%20%28double-precision%29))
  (return 0.0))

(fn TakeDamage
  (params (Damage%20Info :type S%20Damage%20Info%20Structure))
  (return false))