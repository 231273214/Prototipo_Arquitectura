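; BP_Torreta is an enemy turret that turns to face the player character and fires projectiles at a regular interval.
; Tick snaps the actor toward the player each frame, and a Delay in the same chain throttles spawning of BP_Projectile_Enemy at the Point component to every two seconds.
; Each projectile's hit event is bound back to the turret, which sends fixed damage to the hit actor through a TakeDamageMessage call.
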(event Custom|On%20hit
  (params (Other%20Actor :type Actor%20Object%20Reference) (Hit :type Hit%20Result%20Structure))
  (Class|BPIDamageable|TakeDamage(Message) Other%20Actor (Utilities|Struct|MakeS_DamageInfo 1e+01 "NewEnumerator2" "NewEnumerator1")))

(event EventBeginPlay)

(event Collision|EventActorBeginOverlap
  (params (OtherActor :type Actor%20Object%20Reference)))

(event EventTick
  (params (DeltaSeconds :type Float%20%28single-precision%29))
  (Transformation|SetActorRotation (Math|Rotator|FindLookatRotation (Transformation|GetActorLocation) (Transformation|GetActorLocation (Game|GetPlayerCharacter 0))))
  (Utilities|FlowControl|Delay 2.0)
  (bind _returnvalue (Game|SpawnActorfromClass "/Game/TestGame/Systems/ProjectileSystem/BP_Projectile_Enemy.BP_Projectile_Enemy_C" (Transformation|GetWorldTransform (Variables|Default|GetPoint)) "Undefined" "MultiplyWithRoot" 0 0.0 5.0 5e+02 0 false 2e+03 0))
  (EventDispatchers|BindEventtoOnProjectileHit _returnvalue (delegate Custom|On%20hit)))

(fn ConstructionScript)