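; BP_Camera is a camera actor that smoothly follows the player character.
; On BeginPlay it casts player character 0 to BP_Player and stores the reference.
; Every Tick, UpdateCamera moves the actor toward the player's location with VInterpTo at a fixed interpolation speed, without sweeping, giving a lagged follow on position only.
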(event EventBeginPlay
  (bind _asbp_player (Utilities|Casting|CastToBP_Player (Game|GetPlayerCharacter 0)))
  (Variables|Default|SetAs%20BP%20Player _asbp_player))

(event Collision|EventActorBeginOverlap
  (params (OtherActor :type Actor%20Object%20Reference)))

(event EventTick
  (params (DeltaSeconds :type Float%20%28single-precision%29))
  (CallFunction|UpdateCamera))

(fn ConstructionScript)

(fn UpdateCamera
  (Transformation|SetActorLocation (Math|Interpolation|VInterpTo (Transformation|GetActorLocation) (Transformation|GetActorLocation (Variables|Default|GetAs%20BP%20Player)) (Utilities|Time|GetWorldDeltaSeconds) 5.0) false false))